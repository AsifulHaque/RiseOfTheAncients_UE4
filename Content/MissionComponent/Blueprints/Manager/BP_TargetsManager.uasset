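; BP_TargetsManager keeps the list of mission targets for the mission component system.
; Assign_Target adds a target only if no existing entry shares its TargetUniqueName, and Remove_Target deletes the entry found by that name.
; After either change it tells the mission component, when valid, to refresh its current targets.
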(event `Assign_Target`
  (params (TargetInfo :type "/Game/MissionComponent/Blueprints/Structs/MissionComponent/Struct_TargetInfo Structure"))
  (bind _returnvalue (`/Game/MissionComponent/Blueprints/Libraries/MissionSystem/BP_MissionSystemFL.GetMissionComponent`))
  (if (`self.CanAddToTargets?` (`.TargetUniqueName_7_FE44C2044550DF171469159B30339FAA` (break `/Game/MissionComponent/Blueprints/Structs/MissionComponent/Struct_TargetInfo` TargetInfo)))
    (`KismetArrayLibrary.Array_Add` (`self.Targets`) TargetInfo)
    (`/Engine/EditorBlueprintResources/StandardMacros.IsValid` _returnvalue
      (:`Is Valid`
        (`/Game/MissionComponent/Blueprints/Components/BP_MissionComponent.Refresh_Current_Targets` _returnvalue)))))

(event `Remove_Target`
  (params (TargetInfo :type "/Game/MissionComponent/Blueprints/Structs/MissionComponent/Struct_TargetInfo Structure (by ref)"))
  (bind _returnvalue (`/Game/MissionComponent/Blueprints/Libraries/MissionSystem/BP_MissionSystemFL.GetMissionComponent`))
  (`KismetArrayLibrary.Array_Remove` (`self.Targets`) (`self.FindTargetIndex` TargetInfo))
  (`/Engine/EditorBlueprintResources/StandardMacros.IsValid` _returnvalue
    (:`Is Valid`
      (`/Game/MissionComponent/Blueprints/Components/BP_MissionComponent.Refresh_Current_Targets` _returnvalue))))

(fn `CanAddToTargets?`
  (params (WithUniqueName :type Name))
  (returns (CanAdd :type Boolean))
  (locals (LocName :type Name) (LocCanAdd :type Boolean))
  ;[0 0 0 1 16] Check If There Isn't Any With The Same Unique Name
  (set `local.LocName` WithUniqueName)
  (if (!= (`KismetArrayLibrary.Array_Length` (`self.Targets`)) 0)
    (for _array_element (`self.Targets`)
      (if (== (`.TargetUniqueName_7_FE44C2044550DF171469159B30339FAA` (break `/Game/MissionComponent/Blueprints/Structs/MissionComponent/Struct_TargetInfo` _array_element)) (`local.LocName`))
        (set `local.LocCanAdd` false)
        (break)
        (else
          (set `local.LocCanAdd` true))))
    (return (`local.LocCanAdd`))
    (else
      (return true))))

(fn `FindTargetIndex`
  (params (TargetInfo :type "/Game/MissionComponent/Blueprints/Structs/MissionComponent/Struct_TargetInfo Structure (by ref)"))
  (returns (Index :type Integer))
  (locals (LocIndex :type Integer :default 0))
  (for (_array_element _array_index) (`self.Targets`)
    (if (== (`.TargetUniqueName_7_FE44C2044550DF171469159B30339FAA` (break `/Game/MissionComponent/Blueprints/Structs/MissionComponent/Struct_TargetInfo` _array_element)) (`.TargetUniqueName_7_FE44C2044550DF171469159B30339FAA` (break `/Game/MissionComponent/Blueprints/Structs/MissionComponent/Struct_TargetInfo` TargetInfo)))
      (set `local.LocIndex` _array_index)
      (break)
      (else
        (set `local.LocIndex` -1))))
  (return (`local.LocIndex`)))

(fn `UserConstructionScript`)