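; Blueprint interface for the player controller in the mission system, declaring calls that other Blueprints make on it without casting.
; It covers player initialization, building the mission system, requesting the mission component and loading or creating a new game.
; A getter and an updater expose the currently available interaction type as an enum.
; The functions are signatures only, with default return values, so implementing classes supply the logic.
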(fn `BuildMissionSystem`
  (returns (Success :type Boolean))
  (return false))

(fn `GetAvailableInteractionType`
  (returns (InteractionType :type "/Game/MissionComponent/Blueprints/Enums/Common/Enum_InteractionType Enum"))
  (return "NewEnumerator0"))

(fn `InitializePlayer`
  (returns (Success :type Boolean))
  (return false))

(fn `LoadOrCreateNewGame`
  (returns (Success :type Boolean))
  (return false))

(fn `RequestMissionComponent`
  (returns (MissionComponent :type "/Game/MissionComponent/Blueprints/Components/BP_MissionComponent Object Reference"))
  (return null))

(fn `UpdateAvailableInteractionType`
  (params (InteractionType :type "/Game/MissionComponent/Blueprints/Enums/Common/Enum_InteractionType Enum" :default "NewEnumerator0"))
  (returns (Success :type Boolean))
  (return false))