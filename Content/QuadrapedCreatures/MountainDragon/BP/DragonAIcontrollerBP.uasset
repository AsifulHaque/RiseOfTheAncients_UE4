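; AI controller for the mountain dragon that runs its behavior tree and picks which enemy to target.
; On possess it copies fear and chase flags from the Rodent base pawn to the Blackboard.
; Perceived "DragonEnemy" actors and damage causers join an Enemies array.
; Looping timers weight enemies through a distance curve, write the top one to the Blackboard, and prune invalid or expired entries.
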(event `OnTakeAnyDamage_Event` :!signature `self.OnTakeAnyDamage`
  (params (DamagedActor :type "Actor Object Reference") (Damage :type "Float (double-precision)") (DamageType :type "DamageType Object Reference") (InstigatedBy :type "Controller Object Reference") (DamageCauser :type "Actor Object Reference"))
  ;[1 1 1] Bind event if we take any damage add our damager to the Enemies array
  (`self.AddActorToEnemiesArray` DamageCauser))

(event `self.ReceivePossess`
  (params (PossessedPawn :type "Pawn Object Reference"))
  (bind _returnvalue (`self.K2_GetPawn`))
  ;[1 1 1] On Possess
  ;[1 1 1] Run our BehaviorTree
  (`self.RunBehaviorTree` "/Game/QuadrapedCreatures/MountainDragon/BP/DragonBT.DragonBT")
  (`KismetSystemLibrary.Delay` 0.1)
  ;[1 1 1] Set Blackboard Bool "DoIFearTheEnemy?"
  (bind _asbp_npc_rodent_base (cast `/Game/Rodents/ParentClassBlueprints/BP_NPC_Rodent_Base` PossessedPawn))
  (`BlackboardComponent.SetValueAsBool` (`self.Blackboard`) (`self.BlackboardKey_DoIFearTheEnemy?`) (`/Game/Rodents/ParentClassBlueprints/BP_NPC_Rodent_Base.DoIFearEnemies?` _asbp_npc_rodent_base))
  ;[1 1 1] Set BlackboardBool "ChaseTheEnemy?"
  (`BlackboardComponent.SetValueAsBool` (`self.Blackboard`) (`self.BbKey_ChaseTheEnemy?`) (`/Game/Rodents/ParentClassBlueprints/BP_NPC_Rodent_Base.ChaseTheEnemy?` _asbp_npc_rodent_base))
  ;[1 1 1] Remove Expired Enemies -looping timer
  (`KismetSystemLibrary.K2_SetTimer` null "ExpireEnemies" (`self.EnemyExpirationTime`) true)
  ;[1 1 1] EnemySelection- looping timer
  (`KismetSystemLibrary.K2_SetTimer` null "EnemySelection" (`self.EnemyEvaluationFreq`) true)
  ;[1 1 1] Bind event if we take any damage add our damager to the Enemies array
  (`/Engine/EditorBlueprintResources/StandardMacros.IsValid` _returnvalue
    (:`Is Valid`
      (add `self.OnTakeAnyDamage` _returnvalue (delegate `OnTakeAnyDamage_Event`)))))

(event `ExpireEnemies`
  ;[1 1 1] Remove Expired Enemies
  (`self.RemoveExpiredEnemies`))

(event `EnemySelection`
  (bind _enemytarget (`self.EnemyTarget`))
  ;[1 1 1] Enemy Selection
  (`|ExecutionSequence`
    (:`then_0`
      ;;[1 1 1] Get distance to Enemy
      (for (_array_element _array_index) (`self.Enemies`)
        (bind _distancetoenemy (`self.CalculateDistanceToEnemy` _array_element))
        (bind (_actor _weight _lastseen) (break `/Game/Rodents/Rabbit/AI/Rabbit_EnemyStructure` _array_element))
        (`KismetArrayLibrary.Array_Set` (`self.Enemies`) _array_index (make `/Game/Rodents/Rabbit/AI/Rabbit_EnemyStructure` _actor _distancetoenemy _lastseen))))
    (:`then_1`
      ;;[1 1 1] Find our Current Highest Enemy Target
      (set `self.EnemyTarget` null)
      (set `self.CurrentHighestEnemyTarget` 0.0)
      (for _array_element_2 (`self.Enemies`)
        (bind (_actor_2 _weight_2) (break `/Game/Rodents/Rabbit/AI/Rabbit_EnemyStructure` _array_element_2))
        (if (> _weight_2 (`self.CurrentHighestEnemyTarget`))
          (set `self.EnemyTarget` _actor_2)
          (set `self.CurrentHighestEnemyTarget` _weight_2))))
    (:`then_2`
      ;;[1 1 1] Set our highest EnemyTarget as our enemy in the blackboard
      (if (!= (`self.Enemy`) _enemytarget)
        (bind _output_get (set `self.Enemy` _enemytarget))
        (`BlackboardComponent.SetValueAsObject` (`AIBlueprintHelperLibrary.GetBlackboard` null) (`self.BlackboardKey_Enemy`) _output_get)))
    (:`then_3`
      ;;[1 1 1] Set "EnemySpotted?" to true in the Blackboard
      ;; if we have a valid enemy and False if we do not
      (`/Engine/EditorBlueprintResources/StandardMacros.IsValid` (`self.Enemy`)
        (:`Is Valid`
          (`BlackboardComponent.SetValueAsBool` (`self.Blackboard`) (`self.BbKey_EnemySpotted?`) true))
        (:`Is Not Valid`
          (`BlackboardComponent.SetValueAsBool` (`self.Blackboard`) (`self.BbKey_EnemySpotted?`) false))))))

(event `self.AIPerception.OnPerceptionUpdated`
  (params (UpdatedActors :type "Array of Actor Object Reference (by ref)"))
  ;[1 1 1] On Perception Update
  ;[1 1 1] Any Actor with this tag
  (for _array_element UpdatedActors
    (bind _info (`AIPerceptionComponent.GetActorsPerception` (`self.AIPerception`) _array_element))
    (bind _target (break `ActorPerceptionBlueprintInfo` _info))
    (if (`self.ActorHasTag` _target "DragonEnemy")
      ;[1 1 1] Add Actor to the "Enemies" array
      (`self.AddActorToEnemiesArray` _target)
      ;[1 1 1] Bind event if enemy is destroyed-
      ; so we can remove non valad Enemies
      ; from the "Enemies" array
      (add `self.OnDestroyed` _target (delegate `OnEnemyDestroyed`)))))

(event `OnEnemyDestroyed` :!signature `self.OnDestroyed`
  (params (DestroyedActor :type "Actor Object Reference"))
  ;[1 1 1] Bind event if enemy is destroyed-
  ; so we can remove non valad Enemies
  ; from the "Enemies" array
  (`KismetSystemLibrary.CollectGarbage`))

(fn `AddActorToEnemiesArray`
  (params (InputActor :type "Actor Object Reference"))
  (locals (`IsActorInArray?` :type Boolean))
  (bind (_actor _weight) (break `/Game/Rodents/Rabbit/AI/Rabbit_EnemyStructure` (`|GetArrayItem` (`self.Enemies`) (`self.LastSeenIndex`))))
  (`|ExecutionSequence`
    (:`then_0`
      ;[1 1 1] Check if the Actor is already in the "Enemies" array
      (set `local.IsActorInArray?` false)
      (for (_array_element _array_index) (`self.Enemies`)
        (if (== (`.Actor_2_9F3699F344F7A605C2832DA413AE8B60` (break `/Game/Rodents/Rabbit/AI/Rabbit_EnemyStructure` _array_element)) InputActor)
          (set `local.IsActorInArray?` true)
          (set `self.LastSeenIndex` _array_index)
          (break))))
    (:`then_1`
      (if (`local.IsActorInArray?`)
        ;[1 1 1] Actor is in Array, so just reset the last seen time
        (`KismetArrayLibrary.Array_Set` (`self.Enemies`) (`self.LastSeenIndex`) (make `/Game/Rodents/Rabbit/AI/Rabbit_EnemyStructure` _actor _weight))
        (else
          ;[1 1 1] Actor is new, so add it to the "Enemies" array
          (`KismetArrayLibrary.Array_Add` (`self.Enemies`) (make `/Game/Rodents/Rabbit/AI/Rabbit_EnemyStructure` InputActor)))))))

(fn `CalculateDistanceToActor`
  (params (InputActor :type "Actor Object Reference"))
  (returns (DistanceToActor :type "Float (double-precision)"))
  (if (`KismetSystemLibrary.IsValid` InputActor)
    (return (`KismetMathLibrary.VSize` (- (`self.K2_GetActorLocation` InputActor) (`self.K2_GetActorLocation` (`self.K2_GetPawn`)))))
    (else
      (return 2000.0))))

(fn `CalculateDistanceToEnemy`
  (params (ThreatStructureInput :type "/Game/Rodents/Rabbit/AI/Rabbit_EnemyStructure Structure"))
  (returns (DistanceToEnemy :type "Float (double-precision)"))
  (return (`CurveFloat.GetFloatValue` (`self.EnemyDistanceCurve`) (`self.CalculateDistanceToActor` (`.Actor_2_9F3699F344F7A605C2832DA413AE8B60` (break `/Game/Rodents/Rabbit/AI/Rabbit_EnemyStructure` ThreatStructureInput))))))

(fn `RemoveExpiredEnemies`
  (locals (EnemiesToRemove :type "Array of /Game/Rodents/Rabbit/AI/Rabbit_EnemyStructure Structure"))
  (for _array_element (`self.Enemies`)
    (`|ExecutionSequence`
      (:`then_0`
        (bind (_actor _weight _lastseen) (break `/Game/Rodents/Rabbit/AI/Rabbit_EnemyStructure` _array_element))
        ;[1 1 1] Expire this actor if last seen time is more than the "EnemyExpirationTime"
        (if (>= _lastseen (`self.EnemyExpirationTime`))
          (`KismetArrayLibrary.Array_Add` (`local.EnemiesToRemove`) _array_element)))
      (:`then_1`
        ;[1 1 1] Remove any Enemies that are not valid
        (`/Engine/EditorBlueprintResources/StandardMacros.IsValid` _actor
          (:`Is Not Valid`
            (`KismetArrayLibrary.Array_Add` (`local.EnemiesToRemove`) _array_element))))))
  ;[1 1 1] Remove these actors from the "Enemies" array
  (for _array_element_2 (`local.EnemiesToRemove`)
    (`KismetArrayLibrary.Array_RemoveItem` (`self.Enemies`) _array_element_2))
  (`KismetArrayLibrary.Array_Clear` (`local.EnemiesToRemove`)))

(fn `UserConstructionScript`)