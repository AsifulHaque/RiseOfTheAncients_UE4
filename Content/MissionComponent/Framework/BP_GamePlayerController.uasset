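; Player controller that boots the mission system for the local player and routes input for interaction, the quest log and saving.
; BeginPlay caches the controlled Character, triggers the mission build and asks the GameInstance to display a game widget.
; The build loads the first found save or creates a new game, then builds the mission component.
; Helpers track the available interaction type and sphere-trace from the right hand for punches.
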(event `self.ReceiveBeginPlay`
  ;[0 0 0 1 16] Begin Play
  ;;[0 0 0 1 16] Initialize The Player
  (`parent.ReceiveBeginPlay`)
  (if (`self.IsLocalController`)
    (`self.InitializePlayer`)
    ;;[0 0 0 1 16] Custom Event To Build Mission Component
    (message `/Game/MissionComponent/Blueprints/Interfaces/MissionSystem/BP_PlayerControllerInterface.BuildMissionSystem` (`GameplayStatics.GetPlayerController` 0))
    ;;[0 0 0 1 16] To Keep Things In Game Instance
    (message `/Game/MissionComponent/Blueprints/Interfaces/Common/BP_GameInstanceInterface.DisplayGameWidget` (`GameplayStatics.GetGameInstance`) "NewEnumerator3")))

(event `self.ReceivePossess`
  (params (PossessedPawn :type "Pawn Object Reference"))
  ;[0 0 0 1 16] Re-Init On Possess
  (`self.InitializePlayer`))

(event `InputAction|Interact`
  (params (Key :type "Key Structure"))
  ;[1 0 0 1 16] Interaction
  (:`Pressed`
    (`/Game/MissionComponent/Blueprints/Libraries/Common/BP_GameKitFL.RequestInteraction`)))

(event `InputAction|OpenQuestMenu`
  (params (Key :type "Key Structure"))
  ;[1 0 0 1 16] Open Quest Log | Close Binding Is In "Widget_InGameMenu"
  (:`Pressed`
    (`/Game/MissionComponent/Blueprints/Components/BP_MissionComponent.Toggle_Quest_Log` (`/Game/MissionComponent/Blueprints/Libraries/MissionSystem/BP_MissionSystemFL.GetMissionComponent`) "NewEnumerator0")))

(event `InputAction|SaveGame`
  (params (Key :type "Key Structure"))
  ;[1 0 0 1 16] Save Game
  (:`Pressed`
    (`/Game/MissionComponent/Blueprints/Components/BP_MissionComponent.SaveGameOnComponent` (`self.BP_MissionComponent`) true)))

(fn `BuildMissionSystem`
  (returns (Success :type Boolean))
  (`self.LoadOrCreateNewGame`)
  (`/Game/MissionComponent/Blueprints/Components/BP_MissionComponent.Build_Mission_Component` (`self.BP_MissionComponent`))
  (return true))

(fn `GetAvailableInteractionType`
  (returns (InteractionType :type "/Game/MissionComponent/Blueprints/Enums/Common/Enum_InteractionType Enum"))
  (return (`self.AvailableInteractionType`)))

(fn `InitializePlayer`
  (returns (Success :type Boolean))
  ;[0 0 0 1 16] Creates A New Save Game Or Loads The Last Game
  (bind _ascharacter (cast `Character` (`self.K2_GetPawn`))
    (:`then`
      (set `self.ControlledCharacter` _ascharacter)
      (return true))
    (:`CastFailed`
      (return false))))

(fn `LoadOrCreateNewGame`
  (returns (Success :type Boolean))
  (bind _savedslots (`/Game/MissionComponent/Blueprints/Libraries/Common/BP_GameKitFL.FindSavedGames`))
  (if (!= (`KismetArrayLibrary.Array_Length` _savedslots) 0)
    (`/Game/MissionComponent/Blueprints/Components/BP_MissionComponent.Update_New_Game` (`self.BP_MissionComponent`) false)
    (message `/Game/MissionComponent/Blueprints/Interfaces/Common/BP_GameInstanceInterface.LoadSavedGame` (`GameplayStatics.GetGameInstance`) (`|GetArrayItem` _savedslots))
    (return true)
    (else
      (`/Game/MissionComponent/Blueprints/Libraries/Common/BP_GameKitFL.CreateNewGame`)
      (`/Game/MissionComponent/Blueprints/Components/BP_MissionComponent.Update_New_Game` (`self.BP_MissionComponent`) true)
      (return true))))

(fn `RequestMissionComponent`
  (returns (MissionComponent :type "/Game/MissionComponent/Blueprints/Components/BP_MissionComponent Object Reference"))
  (return (`self.BP_MissionComponent`)))

(fn `TraceForPunch`
  (returns (HitActor :type "Actor Object Reference"))
  (bind _returnvalue_location (`KismetMathLibrary.BreakTransform` (`SceneComponent.GetSocketTransform` (`Character.Mesh` (`self.ControlledCharacter`)) "Hand_R" "RTS_World")))
  (bind _outhit (`KismetSystemLibrary.SphereTraceSingle` _returnvalue_location (+ _returnvalue_location (* (`KismetMathLibrary.GetForwardVector` (`self.GetControlRotation`)) 75.0)) 25.0 "TraceTypeQuery1" false (`|MakeArray` self :!type "Actor Object Reference") "ForDuration"))
  (return (`.HitActor` (`GameplayStatics.BreakHitResult` _outhit))))

(fn `UpdateAvailableInteractionType`
  (params (InteractionType :type "/Game/MissionComponent/Blueprints/Enums/Common/Enum_InteractionType Enum" :default "NewEnumerator0"))
  (returns (Success :type Boolean))
  (set `self.AvailableInteractionType` InteractionType)
  (return true))

(fn `UserConstructionScript`)