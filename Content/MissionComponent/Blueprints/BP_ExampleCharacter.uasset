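; Example character Blueprint for the MissionComponent content, providing a punch hit query and gamepad cursor control for menus.
; Every Tick, MoveMouseWithGamepad offsets the mouse position by scaled axis input, with Y inverted, while the in-game menu is open.
; TraceForPunch sphere-traces a short distance from the right-hand socket along the control rotation on the Visibility channel and returns the hit actor, ignoring itself.
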(event `self.ReceiveTick`
  (params (DeltaSeconds :type "Float (single-precision)"))
  ;[0 0 0 1 16] Gamepad Support
  (`self.MoveMouseWithGamepad`))

(fn `MoveMouseWithGamepad`
  (bind (_locationx _locationy) (`PlayerController.GetMousePosition` (`GameplayStatics.GetPlayerController` 0)))
  (if (`/Game/MissionComponent/Blueprints/Libraries/Common/BP_GameKitFL.InGameMenuOpened?`)
    (`PlayerController.SetMouseLocation` (`GameplayStatics.GetPlayerController` 0) (`KismetMathLibrary.FTrunc` (+ (* (`self.GetInputAxisKeyValue`) 15.0) _locationx)) (`KismetMathLibrary.FTrunc` (+ _locationy (* (`self.GetInputAxisKeyValue`) 15.0 -1.0))))))

(fn `TraceForPunch`
  (returns (HitActor :type "Actor Object Reference"))
  (bind _returnvalue_location (`KismetMathLibrary.BreakTransform` (`SceneComponent.GetSocketTransform` (`self.Mesh`) "Hand_R" "RTS_World")))
  (bind _outhit (`KismetSystemLibrary.SphereTraceSingle` _returnvalue_location (+ _returnvalue_location (* (`KismetMathLibrary.GetForwardVector` (`self.GetControlRotation`)) 75.0)) 25.0 "TraceTypeQuery1" false (`|MakeArray` self :!type "Actor Object Reference")))
  (return (`.HitActor` (`GameplayStatics.BreakHitResult` _outhit))))

(fn `UserConstructionScript`)