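; Actor component that gives a Character NPC movement, damage and death handling for the mission system.
; AI MoveTo drives looping random roaming around the start point or indexed paths with per-point speed, delay and reached events.
; At zero health it sends a death message, ragdolls, then after a delay destroys or respawns the owner with its target info.
; Interaction overlap blocks respawn and removal, and can halt roaming.
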(event `self.ReceiveBeginPlay`
  ;[0 0 0 1 16] Set Start Transform On Begin Play
  (set `self.StartTransform` (`Actor.GetTransform` (`self.FindOwnerAI`)))
  ;[0 0 0 1 16] Set Default Speed
  (`self.Adjust_Walk_Speed` (`self.DefaultSpeed`))
  ;[0 0 0 1 16] Move To Random Locations If Requested
  (if (`self.MoveToRandomLocations?`)
    (`self.Move_To_Random_Location` true (`self.RandomLocationRadius`) (`self.RandomLocationDelay`))))

(event `Move_NPC_To`
  (params (Destination :type "Vector Structure"))
  ;[0 0 0 1 16] AI Move To Events
  (`|AIMoveTo` (`self.FindOwnerAI`) Destination null))

(event `Move_To_Random_Location`
  (params (`Loop?` :type Boolean) (Radius :type "Float (double-precision)") (Delay :type "Float (double-precision)"))
  (bind _starttransform_location (`KismetMathLibrary.BreakTransform` (`self.StartTransform`)))
  ;[0 0 0 1 16] AI Move To Events
  (if (`self.CanWalk?`) :!label _label
    (`|AIMoveTo` (`self.FindOwnerAI`) (`NavigationSystemV1.K2_GetRandomLocationInNavigableRadius` _starttransform_location Radius null null) null
      (:`OnSuccess`
        _)
      (:`OnFail`
        _))
    (if `Loop?`
      (`|ExecutionSequence`
        (:`then_0`
          (goto _label_2 :!via `Open`))
        (:`then_1`
          (`/Engine/EditorBlueprintResources/StandardMacros.Gate` true :!label _label_2
            (:`Exit`
              (`KismetSystemLibrary.Delay` Delay)
              (goto _label)))))
      (else
        (goto _label_2 :!via `Close`)))
    (else
      (`KismetSystemLibrary.Delay` 3.0)
      (goto _label))))

(event `Adjust_Walk_Speed`
  (params (WalkSpeed :type "Float (double-precision)"))
  ;[0 0 0 1 16] AI Move To Events
  (set `CharacterMovementComponent.MaxWalkSpeed` WalkSpeed (`Character.CharacterMovement` (`self.FindOwnerAI`))))

(event `Reached_To_Location` :!signature `self.ReachedToLocation`
  (params (WithIndex :type Integer))
  ;[0 0 0 1 16] AI Move To Events
)

(event `Move_NPC_To_Locations`
  (params (LocationInfo :type "Array of /Game/MissionComponent/Blueprints/Structs/MissionComponent/Struct_FollowIndexInfo Structure"))
  ;[0 0 0 1 16] AI Move To Events
  (set `self.LocationInfoToGo` LocationInfo)
  (set `self.CurrentLocationIndex` 0)
  (`self.Start_Follow_The_Path`)
  (add `self.ReachedToLocation` (`|CreateDelegate` :!event `Reached_To_Location`)))

(event `Start_Follow_The_Path`
  (bind _output_delay (break `/Game/MissionComponent/Blueprints/Structs/MissionComponent/Struct_FollowIndexInfo` (`|GetArrayItem` (`self.LocationInfoToGo`) (`self.CurrentLocationIndex`))))
  (bind (_output_delay_2 _output_walkspeed _output_location) (break `/Game/MissionComponent/Blueprints/Structs/MissionComponent/Struct_FollowIndexInfo` (`|GetArrayItem` (`self.LocationInfoToGo`) (`self.CurrentLocationIndex`))))
  ;[0 0 0 1 16] AI Move To Events
  (`self.Adjust_Walk_Speed` _output_walkspeed :!label _label_3)
  (`|AIMoveTo` (`self.FindOwnerAI`) _output_location null
    (:`OnSuccess`
      (`self.ReachedToLocation` (`self.CurrentLocationIndex`))
      (`KismetSystemLibrary.Delay` _output_delay)
      (`/Engine/EditorBlueprintResources/StandardMacros.IncrementInt` (`self.CurrentLocationIndex`)
        (:`  `
          _)))
    (:`OnFail`
      _))
  (if (!= (`KismetArrayLibrary.Array_Length` (`self.LocationInfoToGo`)) (`self.CurrentLocationIndex`))
    (goto _label_3)))

(event `Handle_Damage`
  (params (Damage :type "Float (double-precision)") (DamageType :type "DamageType Object Reference") (InstigatedBy :type "Controller Object Reference") (DamageCauser :type "Actor Object Reference"))
  (bind _returnvalue (`self.FindOwnerAI`))
  (bind _mesh (`Character.Mesh` _returnvalue))
  (bind _returnvalue_2 (`KismetMathLibrary.FClamp` (- (`self.Health`) Damage) 0.0 (`self.Health`)))
  ;[0 0 0 1 16] Handle Death
  (if (`self.CanBeKilled?`)
    (bind _output_get (set `self.Health` _returnvalue_2))
    (`KismetSystemLibrary.PrintString` (`KismetStringLibrary.Conv_DoubleToString` _output_get))
    (if (== _returnvalue_2 0.0)
      (set `self.IsDead?` true)
      (message `/Game/MissionComponent/Blueprints/Interfaces/MissionSystem/BP_AI_Interface.OnDeath` (`self.FindOwnerAI`))
      (`PrimitiveComponent.SetCollisionEnabled` (`Character.CapsuleComponent` _returnvalue) "NoCollision")
      (`SkeletalMeshComponent.SetAllBodiesBelowSimulatePhysics` _mesh "pelvis" true true)
      (`SkeletalMeshComponent.SetAllBodiesBelowPhysicsBlendWeight` _mesh "pelvis" 1.0 false true)
      (`SkeletalMeshComponent.AddImpulseToAllBodiesBelow` _mesh (0.0 0.0 0.0) "pelvis" false true)
      (`PrimitiveComponent.SetCollisionResponseToChannel` _mesh "ECC_Camera" "ECR_Ignore")
      (`PrimitiveComponent.SetCollisionResponseToChannel` _mesh "ECC_PhysicsBody" "ECR_Block")
      (`KismetSystemLibrary.Delay` (`self.RespawnDelay`))
      (if (`self.CanRespawn`) :!label _label_4
        (if (`self.Respawn?`)
          (bind _returnvalue_3 (`|SpawnActorFromClass` (`GameplayStatics.GetObjectClass` (`self.FindOwnerAI`)) (`self.StartTransform`) "AlwaysSpawn" "OverrideRootScale" null null))
          (bind _targetinfo (message `/Game/MissionComponent/Blueprints/Interfaces/MissionSystem/BP_AI_Interface.GetTargetInfo` (`self.FindOwnerAI`)))
          (message `/Game/MissionComponent/Blueprints/Interfaces/MissionSystem/BP_AI_Interface.UpdateTargetInfo` _returnvalue_3 _targetinfo)
          (set `/Game/MissionComponent/Blueprints/Components/BP_AIComponent.Respawn?` (`self.Respawn?`) (`Actor.GetComponentByClass` _returnvalue_3 "BP_AIComponent_C"))
          (`Actor.K2_DestroyActor` (`self.FindOwnerAI`))
          (else
            (`Actor.K2_DestroyActor` (`self.FindOwnerAI`))))
        (else
          (`KismetSystemLibrary.Delay` 1.0)
          (goto _label_4))))))

(event `On_Overlap_To_Interaction`
  ;[0 0 0 1 16] Toggle bCanRespawn On Overlap
  (if (`self.StopOnOverlap?`)
    (`MovementComponent.StopMovementImmediately` (`Character.CharacterMovement` (`self.FindOwnerAI`)))
    (set `self.CanWalk?` false))
  (set `self.CanRespawn` false))

(event `On_End_Overlap_Interaction`
  ;[0 0 0 1 16] Toggle bCanRespawn On Overlap
  (set `self.CanWalk?` true)
  (set `self.CanRespawn` true))

(fn `FindOwnerAI`
  (returns (ReturnValue :type "Character Object Reference"))
  (bind _ascharacter (cast `Character` (`self.GetOwner`)))
  (return _ascharacter))